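; BP_PlatformHigh is a platform prefab that moves between two points and plays a sound when the player character hits it.
; The Construction Script builds two relative InterpToMovement control points from BigLocation and BigLocation2 and sets the travel time from BigDuration.
; A Box hit by ThirdPersonCharacter spawns a sci-fi sweep with random pitch, using the hit's NormalImpulse vector as the sound location rather than the impact point.
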(event OnComponentHit(Box)
  (params (HitComponent :type Primitive%20Component%20Object%20Reference) (OtherActor :type Actor%20Object%20Reference) (OtherComp :type Primitive%20Component%20Object%20Reference) (NormalImpulse :type Vector :default "0, 0, 0") (Hit :type Hit%20Result%20Structure%20%28by%20ref%29))
  (Utilities|Casting|CastToThirdPersonCharacter OtherActor)
  (Audio|SpawnSoundatLocation "/Game/Sounds/interface_sounds/mixkit-sci-fi-sweep-2522.mixkit-sci-fi-sweep-2522" NormalImpulse "0, 0, 0" 2.0 (Math|Random|RandomFloatinRange 0.7 1.0) 0.0 0 0))

(event EventBeginPlay)

(event Collision|EventActorBeginOverlap
  (params (OtherActor :type Actor%20Object%20Reference)))

(event EventTick
  (params (DeltaSeconds :type Float%20%28single-precision%29)))

(fn ConstructionScript
  (bind _interptomovement (Variables|Default|GetInterpToMovement))
  (Variables|/Script/Engine.InterpToMovementComponent|SetControlPoints _interptomovement (Utilities|Array|MakeArray (Utilities|Struct|MakeInterpControlPoint (Variables|Default|GetBigLocation) true) (Utilities|Struct|MakeInterpControlPoint (Variables|Default|GetBigLocation2) true)))
  (Variables|/Script/Engine.InterpToMovementComponent|SetDuration _interptomovement (Variables|Default|GetBigDuration)))